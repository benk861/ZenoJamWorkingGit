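; Checkpoint actor that sets the player's respawn point when the player character overlaps it.
; On overlap it writes RespawnTransform on BP_FirstPersonGameMode, converting the local SpawnTransform location to world space while taking its rotation as-is and forcing unit scale.
; Tick prints CheckpointTime to the screen every frame, and this graph uses that value for nothing else.
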(event `self.ReceiveTick`
  (params (DeltaSeconds :type "Float (single-precision)"))
  (`KismetSystemLibrary.PrintString` (`KismetStringLibrary.Conv_IntToString` (`self.CheckpointTime`))))

(event `self.ReceiveActorBeginOverlap`
  (params (OtherActor :type "Actor Object Reference"))
  (bind (_spawntransform_location _spawntransform_rotation) (`KismetMathLibrary.BreakTransform` (`self.SpawnTransform`)))
  (cast `/Game/FirstPerson/Blueprints/BP_FirstPersonCharacter` (`GameplayStatics.GetPlayerCharacter` 0))
  (if (== OtherActor (`GameplayStatics.GetPlayerCharacter` 0))
    (bind _asbp_first_person_game_mode (cast `/Game/FirstPerson/Blueprints/BP_FirstPersonGameMode` (`GameplayStatics.GetGameMode`)))
    (set `/Game/FirstPerson/Blueprints/BP_FirstPersonGameMode.Respawn Transform` (`KismetMathLibrary.MakeTransform` (`KismetMathLibrary.TransformLocation` (`self.GetTransform`) _spawntransform_location) _spawntransform_rotation) _asbp_first_person_game_mode)))

(fn `UserConstructionScript`)