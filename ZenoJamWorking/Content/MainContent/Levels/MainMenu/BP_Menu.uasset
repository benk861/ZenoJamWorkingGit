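; BP_Menu is a main menu actor that hosts a MainMenu widget in a component and links to other menu actors.
; On BeginPlay it binds to the widget's transition event, which passes an index into its LinkedMenus array.
; A valid index disables its own collision, enables the target menu's, and blends the player's view target to that menu over one second.
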(event `self.ReceiveBeginPlay`
  ;[1 1 1] Transition to other menu
  (bind _asmain_menu (cast `/Game/MainContent/UI/MainMenu` (`WidgetComponent.GetUserWidgetObject` (`self.Widget`))))
  (add `/Game/MainContent/UI/MainMenu.TransitionToLinkedMenu` _asmain_menu (delegate `OnTransitionBetweenMenus`)))

(event `OnTransitionBetweenMenus`
  (params (MenuIndex :type Integer))
  ;[1 1 1] Transition to other menu
  (if (`KismetArrayLibrary.Array_IsValidIndex` (`|MakeArray` (`self.LinkedMenus`)) MenuIndex)
    (`self.TransitionTo` (`|GetArrayItem` (`|MakeArray` (`self.LinkedMenus`)) MenuIndex))))

(event `TransitionTo`
  (params (`New Menu` :type "/Game/MainContent/Levels/MainMenu/BP_Menu Object Reference"))
  (`self.SetActorEnableCollision` false)
  (`self.SetActorEnableCollision` `New Menu` true)
  (`PlayerController.SetViewTargetWithBlend` (`GameplayStatics.GetPlayerController` 0) `New Menu` 1.0 "VTBlend_Linear" 0.0 false))

(fn `UserConstructionScript`)